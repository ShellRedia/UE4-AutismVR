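; InteractManager runs a scripted guide sequence for the VR player, stepping through GuidePlan entries shown on a world-space guide widget.
; Each step sets the widget's image and text, plays its voice clip, and calls an optional function by name via a short timer, such as ShowModelActor or ToNextScene on the game instance.
; Tick turns the widget toward the player pawn and auto-advances when the clip ends on AutoNext steps.
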(event `self.ReceiveBeginPlay`
  (bind _asautism_instance (cast `/Game/Games/AutismInstance` (`GameplayStatics.GetGameInstance`)))
  (set `self.GameIns` _asautism_instance)
  (bind _asvrpawn (cast `/Game/Blueprints/VRPawn` (`GameplayStatics.GetPlayerPawn` 0)))
  (set `self.PlayerPawn` _asvrpawn))

(event `self.ReceiveTick`
  (params (DeltaSeconds :type "Float (single-precision)"))
  (bind _guidewidget (`self.GuideWidget`))
  (`|ExecutionSequence`
    (:`then_0`
      (`SceneComponent.K2_SetWorldRotation` _guidewidget (`KismetMathLibrary.FindLookAtRotation` (`SceneComponent.K2_GetComponentLocation` _guidewidget) (`self.K2_GetActorLocation` (`self.PlayerPawn`))) false false))
    (:`then_1`
      (if (and (`self.PlayNext`) (not (`AudioComponent.IsPlaying` (`self.Audio`))))
        (`self.PlayNextGuideItem`)))))

(fn `PlayNextGuideItem`
  (bind _guideplan (`self.GuidePlan`))
  (bind _guideindex (`self.GuideIndex`))
  (bind (_output_image _output_textcontent _output_textsound _output_optionalfunc _output_autonext) (break `/Game/DataType/EGuide` (`|GetArrayItem` _guideplan _guideindex)))
  (if (< _guideindex (`KismetArrayLibrary.Array_Length` _guideplan))
    (`|ExecutionSequence`
      (:`then_0`
        (set `self.PlayNext` _output_autonext)
        (`AudioComponent.SetSound` (`self.Audio`) _output_textsound)
        (bind _asguide_widget (cast `/Game/UI/GuideWidget` (`WidgetComponent.GetUserWidgetObject` (`self.GuideWidget`))))
        (`/Game/UI/GuideWidget.SetContent` _asguide_widget (make `/Game/DataType/EGuide` _output_image _output_textcontent null))
        (`AudioComponent.Play` (`self.Audio`) 0.0))
      (:`then_1`
        (`KismetSystemLibrary.K2_SetTimer` null _output_optionalfunc 0.2)
        (`/Engine/EditorBlueprintResources/StandardMacros.IncrementInt` (`self.GuideIndex`))))))

(fn `ShowModelActor`
  (`self.SetActorHiddenInGame` (`self.ModelActorRef`) false))

(fn `ToNextScene`
  (`/Game/Games/AutismInstance.To Next Scene` (`self.GameIns`)))

(fn `UserConstructionScript`)