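; PlaceItem is an actor for a pick-up-and-place objective: a scene item spins until caught and must reach its target mesh.
; BlinkTargetItem flashes the target on a looping timer, and Tick detects when the caught item comes close.
; Placement resets and hides the item, shows the target, then reports to AutismInstance, which advances the scene once targets are finished.
; ReplaceItem reattaches the item at its initial location and stops the blink.
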(event `self.ReceiveBeginPlay`
  (set `self.SceneMeshInitLoc` (`SceneComponent.RelativeLocation` (`self.SceneMesh`)))
  (bind _asautism_instance (cast `/Game/Games/AutismInstance` (`GameplayStatics.GetGameInstance`)))
  (set `self.GameIns` _asautism_instance))

(event `self.ReceiveTick`
  (params (DeltaSeconds :type "Float (single-precision)"))
  (bind _gameins (`self.GameIns`))
  (if (`self.IsCaught`)
    (if (`self.IsPlaced`)
      _
      (elif (< (`KismetMathLibrary.Vector_Distance` (`SceneComponent.K2_GetComponentLocation` (`self.SceneMesh`)) (`SceneComponent.K2_GetComponentLocation` (`self.TargetMesh`))) 35.0)
        (set `self.IsPlaced` true)
        (`self.ReplaceItem`)
        (`SceneComponent.SetHiddenInGame` (`self.SceneMesh`) true false)
        (`SceneComponent.SetHiddenInGame` (`self.TargetMesh`) false false)
        (`/Game/Games/AutismInstance.MarkTarget` _gameins (`self.Target_ID`))
        (`/Game/Games/AutismInstance.AddInfo` _gameins "Item placed" (`self.Target_ID`))
        (bind _finished (`/Game/Games/AutismInstance.CheckTargetFinished` _gameins))
        (if _finished
          (`/Game/Games/AutismInstance.To Next Scene` _gameins))))
    (elif (not (`self.IsPlaced`))
      (`SceneComponent.K2_AddLocalRotation` (`self.SceneMesh`) (struct :`Yaw` 0.5) false false))))

(event `BlinkTargetItem`
  (`/Game/Games/AutismInstance.AddInfo` (`self.GameIns`) "Item Caught" (`self.Target_ID`))
  (bind _returnvalue (`KismetSystemLibrary.K2_SetTimerDelegate` (delegate `DoBlink`) 0.3 true))
  (set `self.BlinkTimer` _returnvalue))

(event `DoBlink`
  (bind _targetmesh (`self.TargetMesh`))
  (`SceneComponent.SetHiddenInGame` _targetmesh (not (`SceneComponent.bHiddenInGame` _targetmesh)) false))

(fn `ReplaceItem`
  (bind _scenemesh (`self.SceneMesh`))
  (`/Game/Games/AutismInstance.AddInfo` (`self.GameIns`) "Item Replaced" (`self.Target_ID`))
  (`SceneComponent.K2_DetachFromComponent` _scenemesh "KeepRelative" "KeepRelative" "KeepRelative" true)
  (`SceneComponent.K2_AttachToComponent` _scenemesh (`self.DefaultSceneRoot`) "None" "KeepRelative" "KeepRelative" "KeepRelative" true)
  (`SceneComponent.K2_SetRelativeLocation` _scenemesh (`self.SceneMeshInitLoc`) false false)
  (`KismetSystemLibrary.K2_ClearAndInvalidateTimerHandle` (`self.BlinkTimer`))
  (`SceneComponent.SetHiddenInGame` (`self.TargetMesh`) true false))

(fn `UserConstructionScript`)