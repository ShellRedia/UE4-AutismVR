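; PostureChecker actor that detects hand gestures from the VR player's Oculus body tracking and advances a guided interaction when the expected posture is achieved.
; Each tick it caches world locations of both hands' bones and the model's face sockets.
; Reusable distance-threshold checks detect clasping, thumb-up, index touch and mouth, nose, eye or ear touches.
; CheckAll stores results in PostureAchieved, and the InteractManager's GuideIndex selects which one sets PlayNext.
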(event `self.ReceiveBeginPlay`
  (bind _asvrpawn (cast `/Game/Blueprints/VRPawn` (`GameplayStatics.GetPlayerPawn` 0)))
  (set `self.BodyRef` (`/Game/Blueprints/VRPawn.OculusXRBodyTracking` _asvrpawn)))

(event `self.ReceiveTick`
  (params (DeltaSeconds :type "Float (single-precision)"))
  (bind _interactmanagerref (`self.InteractManagerRef`))
  (`|ExecutionSequence`
    (:`then_0`
      (`KismetArrayLibrary.Array_Clear` (`self.LeftHandBoneLocations`))
      (for _array_element (`self.LeftHandBoneNames`)
        (bind _returnvalue (`PoseableMeshComponent.GetBoneLocationByName` (`self.BodyRef`) _array_element "WorldSpace"))
        (`KismetArrayLibrary.Array_Add` (`self.LeftHandBoneLocations`) _returnvalue)))
    (:`then_1`
      (`KismetArrayLibrary.Array_Clear` (`self.RightHandBoneLocations`))
      (for _array_element_2 (`self.RightHandBoneNames`)
        (bind _returnvalue_2 (`PoseableMeshComponent.GetBoneLocationByName` (`self.BodyRef`) _array_element_2 "WorldSpace"))
        (`KismetArrayLibrary.Array_Add` (`self.RightHandBoneLocations`) _returnvalue_2)))
    (:`then_2`
      (`KismetArrayLibrary.Array_Clear` (`self.FaceSocketLocations`))
      (for _array_element_3 (`self.FaceSocketNames`)
        (`KismetArrayLibrary.Array_Add` (`self.FaceSocketLocations`) (`SceneComponent.GetSocketLocation` (`SkeletalMeshActor.SkeletalMeshComponent` (`self.ModelRef`)) _array_element_3)))
      (if (`|GetArrayItem` (`self.PostureAchieved`) (- (`/Game/Blueprints/InteractManager.GuideIndex` _interactmanagerref) 1)) :!label _label
        (set `/Game/Blueprints/InteractManager.PlayNext` true _interactmanagerref)))
    (:`then_3`
      (`self.CheckAll`)
      (goto _label))))

(fn `CheckAll`
  (`|ExecutionSequence`
    (:`then_0`
      (bind _clasping (`self.IsClasping`)))
    (:`then_1`
      (bind _thumbup (`self.IsThumbUp`)))
    (:`then_2`
      (bind _ok (`self.IsIndexTouch`)))
    (:`then_3`
      (bind _ok_2 (`self.IsMouthTouch`)))
    (:`then_4`
      (bind _ok_3 (`self.IsNoseTouch`)))
    (:`then_5`
      (bind _ok_4 (`self.IsEyeTouch`)))
    (:`then_6`
      (bind _ok_5 (`self.IsEarTouch`)))
    (:`then_7`
      (set `self.PostureAchieved` (`|MakeArray` false _clasping _thumbup _ok false _ok_2 _ok_4 _ok_3 _ok_5 false false false)))))

(fn `DistDisplay`
  (for (_array_element _array_index) (`self.LeftHandBoneLocations`)
    (`KismetSystemLibrary.PrintString` (`KismetStringLibrary.Concat_StrStr` (`KismetStringLibrary.Conv_IntToString` _array_index) " " (`KismetStringLibrary.Conv_DoubleToString` (`KismetMathLibrary.Vector_Distance` (`|GetArrayItem` (`self.RightHandBoneLocations`) _array_index) _array_element))))))

(fn `IsClasping`
  (returns (Clasping :type Boolean))
  (bind _ok (`self.TwoHandsCorrespondingCheck` (`|MakeArray` (make `/Game/DataType/ETwoHandCond` 1 true 4.0) (make `/Game/DataType/ETwoHandCond` 2 true 4.0) (make `/Game/DataType/ETwoHandCond` 3 true 4.0) (make `/Game/DataType/ETwoHandCond` 4 true 4.0) (make `/Game/DataType/ETwoHandCond` 5 true 4.0) (make `/Game/DataType/ETwoHandCond` 6 true 4.0) (make `/Game/DataType/ETwoHandCond` 7 true 5.0) (make `/Game/DataType/ETwoHandCond` 8 true 5.0) :!type "/Game/DataType/ETwoHandCond Structure")))
  (return _ok))

(fn `IsEarTouch`
  (returns (OK :type Boolean))
  (bind _facesocketlocations (`self.FaceSocketLocations`))
  (bind _ok (`self.LocsToLocsCheck` (`|MakeArray` (`|GetArrayItem` (`self.LeftHandBoneLocations`) 4) (`|GetArrayItem` (`self.RightHandBoneLocations`) 4)) (`|MakeArray` (`|GetArrayItem` _facesocketlocations 4) (`|GetArrayItem` _facesocketlocations 5)) false 4.0))
  (return _ok))

(fn `IsEyeTouch`
  (returns (OK :type Boolean))
  (bind _facesocketlocations (`self.FaceSocketLocations`))
  (bind _ok (`self.LocsToLocsCheck` (`|MakeArray` (`|GetArrayItem` (`self.LeftHandBoneLocations`) 4) (`|GetArrayItem` (`self.RightHandBoneLocations`) 4)) (`|MakeArray` (`|GetArrayItem` _facesocketlocations 2) (`|GetArrayItem` _facesocketlocations 3)) false 2.5))
  (return _ok))

(fn `IsIndexTouch`
  (returns (OK :type Boolean))
  (locals (ValidIndex :type "Set of Integer") (Flag :type Boolean :default true))
  (bind _ok (`self.TwoHandsCorrespondingCheck` (`|MakeArray` (make `/Game/DataType/ETwoHandCond` 4 true 3.0) (make `/Game/DataType/ETwoHandCond` 5 false 5.0) (make `/Game/DataType/ETwoHandCond` 7 false 5.0) :!type "/Game/DataType/ETwoHandCond Structure")))
  (return _ok))

(fn `IsMouthTouch`
  (returns (OK :type Boolean))
  (bind _ok (`self.LocsToLocsCheck` (`|MakeArray` (`|GetArrayItem` (`self.LeftHandBoneLocations`) 4) (`|GetArrayItem` (`self.RightHandBoneLocations`) 4)) (`|MakeArray` (`|GetArrayItem` (`self.FaceSocketLocations`))) false 2.5))
  (return _ok))

(fn `IsNoseTouch`
  (returns (OK :type Boolean))
  (bind _ok (`self.LocsToLocsCheck` (`|MakeArray` (`|GetArrayItem` (`self.LeftHandBoneLocations`) 4) (`|GetArrayItem` (`self.RightHandBoneLocations`) 4)) (`|MakeArray` (`|GetArrayItem` (`self.FaceSocketLocations`) 1)) false 2.5))
  (return _ok))

(fn `IsThumbUp`
  (returns (ThumbUp :type Boolean))
  (locals (Flag :type Boolean :default true) (SimilarIndex_A :type "Array of Integer") (SimilarIndex_B :type "Array of Integer") (UnsimilarIndex_A :type "Array of Integer") (UnsimilarIndex_B :type "Array of Integer") (CheckList :type "Array of /Game/DataType/EOneHandCond Structure"))
  (bind _checklist (`local.CheckList`))
  (bind _ok (`self.OneHandsCorrespondingCheck` _checklist (`self.LeftHandBoneLocations`)))
  (bind _ok_2 (`self.OneHandsCorrespondingCheck` _checklist (`self.RightHandBoneLocations`)))
  (return (or _ok_2 _ok)))

(fn `LocsToLocsCheck`
  (params (Locations1 :type "Array of Vector Structure") (Locations2 :type "Array of Vector Structure") (Greater :type Boolean) (Limit :type "Float (double-precision)"))
  (returns (OK :type Boolean))
  (locals (Flag :type Boolean :default false))
  (for _array_element Locations1
    (for _array_element_2 Locations2
      (if Greater
        (bind _returnvalue (`KismetMathLibrary.Vector_Distance` _array_element_2 _array_element))
        (if (> _returnvalue Limit)
          (set `local.Flag` true :!label _label))
        (elif (< _returnvalue Limit)
          (goto _label)))))
  (return (`local.Flag`)))

(fn `OneHandsCorrespondingCheck`
  (params (CheckList :type "Array of /Game/DataType/EOneHandCond Structure") (HandBoneLocations :type "Array of Vector Structure"))
  (returns (OK :type Boolean))
  (locals (Flag :type Boolean :default true))
  (for _array_element CheckList
    (if (`.IsGreater_8_3F69D1324C09FAEAFB94769A3858F122` (break `/Game/DataType/EOneHandCond` _array_element))
      (bind _returnvalue (`KismetMathLibrary.Vector_Distance` (`|GetArrayItem` HandBoneLocations (break `/Game/DataType/EOneHandCond` _array_element)) (`|GetArrayItem` HandBoneLocations (`.Index_2_4_FC1B94AD4EF3FD81583DA097D1627AD0` (break `/Game/DataType/EOneHandCond` _array_element)))))
      (if (> _returnvalue (`.Limit_11_45BC2EAA489F12E6BB3233BD5E6ACCF0` (break `/Game/DataType/EOneHandCond` _array_element)))
        (set `local.Flag` false :!label _label))
      (elif (< _returnvalue _returnvalue)
        (goto _label))))
  (return (`local.Flag`)))

(fn `TwoHandsCorrespondingCheck`
  (params (CheckList :type "Array of /Game/DataType/ETwoHandCond Structure"))
  (returns (OK :type Boolean))
  (locals (Flag :type Boolean :default true))
  (for _array_element CheckList
    (if (`.IsGreater_5_37C23E3B4AD7F030658E81A9532524FA` (break `/Game/DataType/ETwoHandCond` _array_element))
      (bind _returnvalue (`KismetMathLibrary.Vector_Distance` (`|GetArrayItem` (`self.LeftHandBoneLocations`) (break `/Game/DataType/ETwoHandCond` _array_element)) (`|GetArrayItem` (`self.RightHandBoneLocations`) (break `/Game/DataType/ETwoHandCond` _array_element))))
      (if (> _returnvalue (`.Limit_8_CCFC6BC8457B4185193A1C8B9F548F21` (break `/Game/DataType/ETwoHandCond` _array_element)))
        (set `local.Flag` false :!label _label))
      (elif (< _returnvalue (`.Limit_8_CCFC6BC8457B4185193A1C8B9F548F21` (break `/Game/DataType/ETwoHandCond` _array_element)))
        (goto _label))))
  (return (`local.Flag`)))

(fn `UserConstructionScript`)